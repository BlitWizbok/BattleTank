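; BP_Tank is a tank Blueprint that currently handles only aiming of its spring-arm camera.
; The AimAzimuth and AimElevation axis inputs add local yaw and pitch rotation to the SpringArm.
; Small helper graphs scale input by Sensitivity and world delta seconds for frame-rate-independent turning.
; The construction script is empty, and the graphs contain no movement or firing logic.
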(event `InputAxis|AimAzimuth`
  (params (AxisValue :type "Float (single-precision)"))
  ;[1 0 0.8342 0.5] Camera Input Bindings
  (`SceneComponent.K2_AddLocalRotation` (`self.SpringArm`) (`KismetMathLibrary.MakeRotator` 0.0 0.0 (* (`self.MultiplyDeltaTime` AxisValue) (`self.Sensitivity`))) false false))

(event `InputAxis|AimElevation`
  (params (AxisValue :type "Float (single-precision)"))
  ;[1 0 0.8342 0.5] Camera Input Bindings
  (`SceneComponent.K2_AddLocalRotation` (`self.SpringArm`) (`KismetMathLibrary.MakeRotator` 0.0 (* (`self.MultiplyDeltaTime` AxisValue) (`self.Sensitivity`))) false false))

(fn `UserConstructionScript`)